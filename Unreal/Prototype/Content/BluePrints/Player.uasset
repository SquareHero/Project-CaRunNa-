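; Player is a setup Blueprint that spawns local players for multiplayer when play begins.
; On BeginPlay it creates players for four fixed controller IDs and sets focus to the game viewport.
; It then loops up to PlayerMax, offsetting each player pawn along the X axis by its index so the pawns are spread apart.
; Tick, overlap and construction logic are empty.
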(event `self.ReceiveBeginPlay`
  ;[1 1 1] CeatePlayer
  (`GameplayStatics.CreatePlayer` 0)
  (`GameplayStatics.CreatePlayer` 1)
  (`GameplayStatics.CreatePlayer` 2)
  (`GameplayStatics.CreatePlayer` 3)
  (`WidgetBlueprintLibrary.SetFocusToGameViewport`)
  (for _index (range (`self.PlayerMax`))
    (bind _returnvalue (`GameplayStatics.GetPlayerPawn` _index))
    (`self.K2_SetActorLocation` _returnvalue (+ (`self.K2_GetActorLocation` _returnvalue) (* (100.0 0.0 0.0) _index)) false false)))

(fn `UserConstructionScript`)